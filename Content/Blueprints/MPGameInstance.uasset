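; Game instance Blueprint that handles LAN multiplayer sessions through host, search, join and destroy events.
; Hosting creates a session, then opens ThirdPersonExampleMap as a listen server via a console command.
; Searching requests a single result and stores it in SessionResult, which joining uses by taking the first entry without checking it.
; Outcomes are mostly reported with on-screen debug strings, though a successful search prints nothing.
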(event `HostGame`
  (bind _returnvalue (`GameplayStatics.GetPlayerController` 0))
  ;[1 1 1] Host Game
  (`CreateSessionCallbackProxy.CreateSession` _returnvalue 0 true
    (:`OnSuccess`
      (`KismetSystemLibrary.ExecuteConsoleCommand` "open ThirdPersonExampleMap?listen" _returnvalue)
      (`KismetSystemLibrary.PrintString` "Session Created"))
    (:`OnFailure`
      (`KismetSystemLibrary.PrintString` "failed to create session"))))

(event `SearchForGame`
  ;[1 1 1] Find Games
  (bind _results (`FindSessionsCallbackProxy.FindSessions` (`GameplayStatics.GetPlayerController` 0) 1 true)
    (:`OnSuccess`
      (set `self.SessionResult` _results))
    (:`OnFailure`
      (`KismetSystemLibrary.PrintString` "failed to find games"))))

(event `JoinGame`
  ;[1 1 1] Join Game
  (`JoinSessionCallbackProxy.JoinSession` (`GameplayStatics.GetPlayerController` 0) (`KismetArrayLibrary.Array_Get` (`self.SessionResult`))
    (:`OnSuccess`
      (`KismetSystemLibrary.PrintString` "joining session"))
    (:`OnFailure`
      (`KismetSystemLibrary.PrintString` "failed to join session"))))

(event `DestroyGame`
  ;[1 1 1] Destroy Game Session
  (`DestroySessionCallbackProxy.DestroySession` (`GameplayStatics.GetPlayerController` 0)
    (:`OnSuccess`
      (`KismetSystemLibrary.PrintString` "successfully destroyed session"))
    (:`OnFailure`
      (`KismetSystemLibrary.PrintString` "error destroying session"))))